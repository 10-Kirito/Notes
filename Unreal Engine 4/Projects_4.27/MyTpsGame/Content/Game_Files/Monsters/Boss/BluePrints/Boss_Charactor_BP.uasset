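; Boss monster character that wanders the navmesh at random until damaged, then chases and attacks the player.
; Chase and attack montage alternate through AI MoveTo, returning to wandering when Tick reports the player dead.
; Attack_ball overlaps send damage to the player only while AttackState, toggled by AttackPlayer and EndAttackPlayer, is on.
; Damage updates the BossUI health bar; death stops movement, hides the widget and destroys the actor after a delay.
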(event OnComponentBeginOverlap(attack_ball)
  (params (OverlappedComponent :type Primitive%20Component%20Object%20Reference) (OtherActor :type Actor%20Object%20Reference) (OtherComp :type Primitive%20Component%20Object%20Reference) (OtherBodyIndex :type Integer) (bFromSweep :type Boolean) (SweepResult :type Hit%20Result%20Structure%20%28by%20ref%29))
  ;[1 1 1] 当玩家碰到爪子的时候后，怪物对其造成伤害
  (if (Variables|Default|GetAttackState)
    (bind _astps_charactor_bp (Utilities|Casting|CastToTps_Charactor_BP OtherActor))
    (bind _output_get (Variables|Default|SetAttackedPlayer _astps_charactor_bp))
    (Class|DamageInterface|TakeDamage(Message) _output_get (Variables|Default|GetAttackDamage))))

(event OnComponentEndOverlap(attack_ball)
  (params (OverlappedComponent :type Primitive%20Component%20Object%20Reference) (OtherActor :type Actor%20Object%20Reference) (OtherComp :type Primitive%20Component%20Object%20Reference) (OtherBodyIndex :type Integer)))

(event Custom|Boss_Move
  (if (not (Variables|Default|GetisDeath))
    ;[1 1 1] AI控制Boss移动
    (AI|AIMoveTo self (.RandomLocation (Class|NavigationSystemV1|GetRandomPointinNavigableRadius (Transformation|GetActorLocation) 1e+05 0 "/Script/AIModule.NavFilter_AIControllerDefault")) 0 5.0 false
      (:OnSuccess
        (CallFunction|BossMove)))))

(event Custom|AI攻击玩家
  ;[1 1 1] 实现AI攻击玩家
  (if (not (Variables|Default|GetisDeath))
    (if (Variables|Default|GetPlayerDeath)
      (CallFunction|BossMove)
      (else
        (bind _returnvalue (Animation|PlayAnimMontage "/Game/Game_Files/Monsters/Boss/Animitions/Attack_Montage.Attack_Montage" 1.0 "None"))
        (Utilities|FlowControl|Delay _returnvalue)
        (CallFunction|追捕玩家)))))

(event Custom|AttackPlayer
  (Variables|Default|SetAttackState true))

(event Custom|EndAttackPlayer
  (Variables|Default|SetAttackState false))

(event Custom|追捕玩家
  ;[1 1 1] 追捕玩家
  (if (not (Variables|Default|GetisDeath))
    (Variables|/Script/Engine.CharacterMovementComponent|SetMaxWalkSpeed (Variables|Character|GetCharacterMovement) 3e+02)
    (AI|AIMoveTo self "0, 0, 0" (Game|Player|GetPlayerPawn 0) 5.0 false
      (:OnSuccess
        (CallFunction|AI攻击玩家))
      (:OnFail
        (CallFunction|追捕玩家)))))

(event EventBeginPlay
  ;[1 1 1] AI控制Boss移动
  (CallFunction|BossMove)
  (Variables|Default|SetCurrentHealth (Variables|Default|GetMaxHealth))
  (CallFunction|UIUpdate))

(event Collision|EventActorBeginOverlap
  (params (OtherActor :type Actor%20Object%20Reference)))

(event EventTakeDamage
  (params (Damage :type Float%20%28single-precision%29))
  ;[1 1 1] 对接口进行重写
  (bind _output_get (Variables|Default|SetCurrentHealth (- (Variables|Default|GetCurrentHealth) Damage)))
  (CallFunction|UIUpdate)
  (if (<= _output_get 0.0)
    (Variables|Default|SetisDeath true)
    (Components|Movement|StopMovementImmediately (Variables|Character|GetCharacterMovement))
    (Rendering|SetVisibility (Variables|Default|GetWidget) false false)
    (Utilities|FlowControl|Delay 8.0)
    (Actor|DestroyActor)
    (else
      (CallFunction|追捕玩家))))

(event EventTick
  (params (DeltaSeconds :type Float%20%28single-precision%29))
  ;[1 1 1] 获取玩家死亡状态
  (bind _astps_charactor_bp (Utilities|Casting|CastToTps_Charactor_BP (Game|GetPlayerCharacter 0)))
  (Variables|Default|SetPlayerDeath (Variables|/Game/Game_Files/Charactor/Tps_Charactor_BP.Tps_Charactor_BP_C|GetDeath _astps_charactor_bp)))

(fn ConstructionScript)

(fn UIUpdate
  ;[1 1 1] 更新Boss血量
  (bind _asboss_ui (Utilities|Casting|CastToBossUI (UserInterface|GetUserWidgetObject (Variables|Default|GetWidget))))
  (bind _output_get (LocalVariables|SetBossUI _asboss_ui))
  (Progress|SetPercent (Variables|/Game/Game_Files/Monsters/Boss/BluePrints/BossUI.BossUI_C|GetHealth _output_get) (/ (Variables|Default|GetCurrentHealth) (Variables|Default|GetMaxHealth))))