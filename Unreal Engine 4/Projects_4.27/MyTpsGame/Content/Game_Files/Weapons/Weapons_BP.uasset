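; Weapon actor that the third-person character can pick up, with its stats, sounds and montages held in a WeaponInfo struct.
; Sphere overlap with Tps_Charactor_BP stores the character, enables input and shows a PickUpUI widget with weapon name and icon; leaving hides it.
; Pressing F in range passes the weapon to the character's 捡取武器, while CloseComponent separately disables the sphere and widget.
; The construction script writes the actor's own class into WeaponInfo.
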(event OnComponentBeginOverlap(Sphere)
  (params (OverlappedComponent :type Primitive%20Component%20Object%20Reference) (OtherActor :type Actor%20Object%20Reference) (OtherComp :type Primitive%20Component%20Object%20Reference) (OtherBodyIndex :type Integer) (bFromSweep :type Boolean) (SweepResult :type Hit%20Result%20Structure%20%28by%20ref%29))
  (bind _widget (Variables|Default|GetWidget))
  (bind _weaponinfo (Variables|Default|GetWeaponInfo))
  (bind (_武器名称 _图标) (Utilities|Struct|BreakWeapon_Info _weaponinfo))
  (bind _returnvalue (UserInterface|GetUserWidgetObject _widget))
  (bind _aspick_up_ui (Utilities|Casting|CastToPickUpUI _returnvalue))
  ;[1 1 1] 这里获得碰撞对象的引用之后，我们需要将其存储起来，以备后面使用
  (bind _astps_charactor_bp (Utilities|Casting|CastToTps_Charactor_BP OtherActor))
  (Variables|Default|SetPickedMan _astps_charactor_bp)
  (Variables|Default|SetCanPickUp? true) ; 如果人物接近武器的话，就可以\n捡起来武器
  (Rendering|SetVisibility (Variables|Default|GetWidget) true false)
  (Input|EnableInput (Game|GetPlayerController 0))
  ;[1 1 1] 获得我们的UI类引用
  (Variables|/Game/Game_Files/UI/PickUpUI.PickUpUI_C|Set武器名字 _aspick_up_ui (Utilities|Text|ToText(String) _武器名称))
  (Variables|/Game/Game_Files/UI/PickUpUI.PickUpUI_C|Set武器图标 _aspick_up_ui _图标))

(event OnComponentEndOverlap(Sphere)
  (params (OverlappedComponent :type Primitive%20Component%20Object%20Reference) (OtherActor :type Actor%20Object%20Reference) (OtherComp :type Primitive%20Component%20Object%20Reference) (OtherBodyIndex :type Integer))
  ;[1 1 1] 当人物离开之后，就将指定的变量置空即可
  (bind _astps_charactor_bp (Utilities|Casting|CastToTps_Charactor_BP OtherActor))
  (Variables|Default|SetPickedMan _astps_charactor_bp)
  (Variables|Default|SetCanPickUp? false) ; 如果人物离开武器，就不可以捡起武器
  (Rendering|SetVisibility (Variables|Default|GetWidget) false false))

(event Custom|CloseComponent
  ;[1 1 1] 该事件的目的是为了当人物捡起来武器之后，取消枪械的碰撞体以及Widget显示信息
  (Collision|SetCollisionEnabled (Variables|Default|GetSphere) "NoCollision")
  (Rendering|SetVisibility (Variables|Default|GetWidget) false false))

(event EventBeginPlay)

(event Collision|EventActorBeginOverlap
  (params (OtherActor :type Actor%20Object%20Reference)))

(event EventTick
  (params (DeltaSeconds :type Float%20%28single-precision%29)))

(event Input|KeyboardEvents|F
  (params (Key :type Key%20Structure :default "None"))
  (bind _pickedman (Variables|Default|GetPickedMan))
  ;[1 1 1] 按键F，实现功能捡起武器
  (:Pressed
    (Utilities|IsValid _pickedman
      (:Is%20Valid
        (if (Variables|Default|GetCanPickUp?)
          (Default|捡取武器 _pickedman self))))))

(fn ConstructionScript
  ;[1 1 1] 结构体的默认构造函数
  (Variables|Default|SetWeaponInfo (Utilities|Struct|MakeWeapon_Info (.weapontype (Variables|Default|GetWeaponInfo)) (.武器名称 (Variables|Default|GetWeaponInfo)) (Utilities|GetClass self) (.图标 (Variables|Default|GetWeaponInfo)) (.射击速度 (Variables|Default|GetWeaponInfo)) (.开火声音 (Variables|Default|GetWeaponInfo)) (.当前弹夹子弹数 (Variables|Default|GetWeaponInfo)) (.弹夹载弹量 (Variables|Default|GetWeaponInfo)) (.当前总子弹数 (Variables|Default|GetWeaponInfo)) (.武器伤害值 (Variables|Default|GetWeaponInfo)) (.weaponholdsocket (Variables|Default|GetWeaponInfo)) (.weaponequipsocket (Variables|Default|GetWeaponInfo)) (.装备声音 (Variables|Default|GetWeaponInfo)) (.拾取武器声音 (Variables|Default|GetWeaponInfo)) (.武器空弹声音 (Variables|Default|GetWeaponInfo)) (.射击距离 (Variables|Default|GetWeaponInfo)) (.武器使用弹药类型 (Variables|Default|GetWeaponInfo)) (.射击montage (Variables|Default|GetWeaponInfo)) (.武器重装弹药montage (Variables|Default|GetWeaponInfo)))))